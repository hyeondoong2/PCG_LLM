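; BP_PCG is a Blueprint that drives a PCG component's tree density from biome keywords in the LLMInput string.
; Every Tick it checks for "Forest" or "Desert", picks a dense or sparse TreeDensity, then cleans up and regenerates the graph.
; The float graph parameter is set after the Generate call, and only the Desert branch names it Tree_Density.
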(event EventBeginPlay)

(event Collision|EventActorBeginOverlap
  (params (OtherActor :type Actor%20Object%20Reference)))

(event EventTick
  (params (DeltaSeconds :type Float%20%28single-precision%29))
  (bind _pcg (Variables|Default|GetPCG))
  (bind _pcg_2 (Variables|Default|GetPCG))
  (if (Utilities|String|Contains (Variables|Default|GetLLM_Input) "Forest")
    (bind _output_get (Variables|Default|SetTree_Density 1.0))
    (Class|PCGComponent|Cleanup _pcg_2 true)
    (PCG|Generate _pcg_2 true)
    (Effects|Components|ParticleSystem|SetFloatParameter (Variables|/Script/PCG.PCGComponent|GetGraphInstance _pcg_2) "Tree_Density" _output_get)
    (elif (Utilities|String|Contains (Variables|Default|GetLLM_Input) "Desert")
      (bind _output_get_2 (Variables|Default|SetTree_Density 0.1))
      (Class|PCGComponent|Cleanup _pcg true)
      (PCG|Generate _pcg true)
      (Effects|Components|ParticleSystem|SetFloatParameter (Variables|/Script/PCG.PCGComponent|GetGraphInstance _pcg) "Tree_Density" _output_get_2))))

(fn ConstructionScript)