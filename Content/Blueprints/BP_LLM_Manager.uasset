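; Manager actor that applies map parameters, apparently LLM-generated, to level difficulty, lighting and procedural layout.
; A DoOnce on Tick leads into binding the params-received event, whose chain prints the analysis and stores spawn rate, complexity, difficulty, aggression and obstacle type.
; The atmosphere tag selects the directional light's color (dark foggy, bright clear or red alarm), and each match then cleans up and regenerates PCG.
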(event Custom|OnMapParamsReceived_Event
  (params (MapParams :type LLM%20Map%20Params%20Structure%20%28by%20ref%29))
  (bind (_analysis _difficultymultiplier _enemyspawnrate _enemyaggressiontag _mapcomplexity _obstacletypetag _atmospheretag) (Utilities|Struct|BreakLLMMapParams MapParams))
  (bind _pcg (Variables|Default|GetPCG))
  (EventDispatchers|BindEventtoOnMapParamsReceived (delegate Custom|OnMapParamsReceived_Event))
  (Development|PrintString _analysis)
  (Variables|Default|SetCurrentSpawnRate _enemyspawnrate)
  (Variables|Default|SetTargetComplexity _mapcomplexity)
  (Variables|Default|SetCurrentDifficulty _difficultymultiplier)
  (Development|PrintText (Utilities|Text|ToText(Float) _difficultymultiplier "HalfToEven") true true "(R=0.000000,G=0.660000,B=1.000000,A=1.000000)" _difficultymultiplier)
  (Variables|Default|SetCurrentAggression (GameplayTags|GetTagName _enemyaggressiontag))
  (Variables|Default|SetCurrentObstacleType (GameplayTags|GetTagName _obstacletypetag))
  (bind _returnvalue (Actor|GetActorOfClass "/Script/Engine.DirectionalLight"))
  (switch string (Utilities|String|ToString(Name) (GameplayTags|GetTagName _atmospheretag))
    (:Dark_Foggy
      (Rendering|Components|Light|SetIntensity (Variables|/Script/Engine.Light|GetLightComponent _returnvalue) 3.0)
      (Rendering|Components|Light|SetLightColor (Variables|/Script/Engine.Light|GetLightComponent _returnvalue) "(R=0.004062,G=0.019997,B=0.177083,A=1.000000)" true))
    (:Bright_Clear
      (Rendering|Components|Light|SetIntensity (Variables|/Script/Engine.Light|GetLightComponent _returnvalue) 3.0)
      (Rendering|Components|Light|SetLightColor (Variables|/Script/Engine.Light|GetLightComponent _returnvalue) "(R=1.000000,G=1.000000,B=1.000000,A=1.000000)" true))
    (:Red_Alarm
      (Rendering|Components|Light|SetIntensity (Variables|/Script/Engine.Light|GetLightComponent _returnvalue) 3.0)
      (Rendering|Components|Light|SetLightColor (Variables|/Script/Engine.Light|GetLightComponent _returnvalue) "(R=1.000000,G=0.019997,B=0.000000,A=1.000000)" true)))
  (Class|PCGComponent|Cleanup _pcg false)
  (PCG|Generate _pcg false))

(event EventBeginPlay)

(event Collision|EventActorBeginOverlap
  (params (OtherActor :type Actor%20Object%20Reference)))

(event EventTick
  (params (DeltaSeconds :type Float%20%28single-precision%29))
  (bind _pcg (Variables|Default|GetPCG))
  (Utilities|FlowControl|DoOnce false
    (:Completed
      (EventDispatchers|BindEventtoOnMapParamsReceived (delegate Custom|OnMapParamsReceived_Event))
      (Development|PrintString (.Analysis (Utilities|Struct|BreakLLMMapParams (stale Custom|OnMapParamsReceived_Event MapParams))))
      (Variables|Default|SetCurrentSpawnRate (.EnemySpawnRate (Utilities|Struct|BreakLLMMapParams (stale Custom|OnMapParamsReceived_Event MapParams))))
      (Variables|Default|SetTargetComplexity (.MapComplexity (Utilities|Struct|BreakLLMMapParams (stale Custom|OnMapParamsReceived_Event MapParams))))
      (Variables|Default|SetCurrentDifficulty (.DifficultyMultiplier (Utilities|Struct|BreakLLMMapParams (stale Custom|OnMapParamsReceived_Event MapParams))))
      (Development|PrintText (Utilities|Text|ToText(Float) (.DifficultyMultiplier (Utilities|Struct|BreakLLMMapParams (stale Custom|OnMapParamsReceived_Event MapParams))) "HalfToEven") true true "(R=0.000000,G=0.660000,B=1.000000,A=1.000000)" (.DifficultyMultiplier (Utilities|Struct|BreakLLMMapParams (stale Custom|OnMapParamsReceived_Event MapParams))))
      (Variables|Default|SetCurrentAggression (GameplayTags|GetTagName (.EnemyAggressionTag (Utilities|Struct|BreakLLMMapParams (stale Custom|OnMapParamsReceived_Event MapParams)))))
      (Variables|Default|SetCurrentObstacleType (GameplayTags|GetTagName (.ObstacleTypeTag (Utilities|Struct|BreakLLMMapParams (stale Custom|OnMapParamsReceived_Event MapParams)))))
      (bind _returnvalue (Actor|GetActorOfClass "/Script/Engine.DirectionalLight"))
      (switch string (Utilities|String|ToString(Name) (GameplayTags|GetTagName (.AtmosphereTag (Utilities|Struct|BreakLLMMapParams (stale Custom|OnMapParamsReceived_Event MapParams)))))
        (:Dark_Foggy
          (Rendering|Components|Light|SetIntensity (Variables|/Script/Engine.Light|GetLightComponent _returnvalue) 3.0)
          (Rendering|Components|Light|SetLightColor (Variables|/Script/Engine.Light|GetLightComponent _returnvalue) "(R=0.004062,G=0.019997,B=0.177083,A=1.000000)" true))
        (:Bright_Clear
          (Rendering|Components|Light|SetIntensity (Variables|/Script/Engine.Light|GetLightComponent _returnvalue) 3.0)
          (Rendering|Components|Light|SetLightColor (Variables|/Script/Engine.Light|GetLightComponent _returnvalue) "(R=1.000000,G=1.000000,B=1.000000,A=1.000000)" true))
        (:Red_Alarm
          (Rendering|Components|Light|SetIntensity (Variables|/Script/Engine.Light|GetLightComponent _returnvalue) 3.0)
          (Rendering|Components|Light|SetLightColor (Variables|/Script/Engine.Light|GetLightComponent _returnvalue) "(R=1.000000,G=0.019997,B=0.000000,A=1.000000)" true)))
      (Class|PCGComponent|Cleanup _pcg false)
      (PCG|Generate _pcg false))))

(fn ConstructionScript)